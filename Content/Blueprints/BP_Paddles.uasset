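; BP_Paddles holds the left and right paddles for a two-player game and moves them vertically from player input.
; The P1 Move and P2 Move axis events each offset their cube along local Z by the axis value times MovementSpeed.
; After each move, the cube's world Z is clamped between TopBound and BottomBound.
; Movement is applied per input event without delta-time scaling, so speed depends on frame rate.
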(event `InputAxis|P1 Move`
  (params (AxisValue :type "Float (single-precision)"))
  (bind (_returnvalue_x _returnvalue_y _returnvalue_z) (`KismetMathLibrary.BreakVector` (`SceneComponent.K2_GetComponentLocation` (`self.CubeLeft`))))
  (bind (_returnvalue_x_2 _returnvalue_y_2 _returnvalue_z_2) (`KismetMathLibrary.BreakVector` (`SceneComponent.K2_GetComponentLocation` (`self.CubeLeft`))))
  (`SceneComponent.K2_AddLocalOffset` (`self.CubeLeft`) (`KismetMathLibrary.MakeVector` 0.0 0.0 (* (`self.MovementSpeed`) (`self.GetInputAxisValue`))) false false)
  (if (> _returnvalue_z (`self.TopBound`))
    (`SceneComponent.K2_SetWorldLocation` (`self.CubeLeft`) (`KismetMathLibrary.MakeVector` _returnvalue_x _returnvalue_y (`self.TopBound`)) false false)
    (elif (< _returnvalue_z_2 (`self.BottomBound`))
      (`SceneComponent.K2_SetWorldLocation` (`self.CubeLeft`) (`KismetMathLibrary.MakeVector` _returnvalue_x_2 _returnvalue_y_2 (`self.BottomBound`)) false false))))

(event `InputAxis|P2 Move`
  (params (AxisValue :type "Float (single-precision)"))
  (bind (_returnvalue_x _returnvalue_y _returnvalue_z) (`KismetMathLibrary.BreakVector` (`SceneComponent.K2_GetComponentLocation` (`self.CubeRight`))))
  (bind (_returnvalue_x_2 _returnvalue_y_2 _returnvalue_z_2) (`KismetMathLibrary.BreakVector` (`SceneComponent.K2_GetComponentLocation` (`self.CubeRight`))))
  (`SceneComponent.K2_AddLocalOffset` (`self.CubeRight`) (`KismetMathLibrary.MakeVector` 0.0 0.0 (* (`self.MovementSpeed`) (`self.GetInputAxisValue`))) false false)
  (if (> _returnvalue_z_2 (`self.TopBound`))
    (`SceneComponent.K2_SetWorldLocation` (`self.CubeRight`) (`KismetMathLibrary.MakeVector` _returnvalue_x_2 _returnvalue_y_2 (`self.TopBound`)) false false)
    (elif (< _returnvalue_z (`self.BottomBound`))
      (`SceneComponent.K2_SetWorldLocation` (`self.CubeRight`) (`KismetMathLibrary.MakeVector` _returnvalue_x _returnvalue_y (`self.BottomBound`)) false false))))

(fn `UserConstructionScript`)