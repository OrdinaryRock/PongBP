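; BP_Ball is a Pong-style ball that moves in the XZ plane and bounces between paddles and height limits.
; BeginPlay builds a randomly signed X and Z velocity from a speed range and multiplier, and Tick applies it as a swept local offset.
; Hitting a BP_Paddles actor flips X velocity, while passing the fixed upper or lower Z bound flips Z velocity.
; A random-rotation branch is left unconnected.
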(event `self.ReceiveBeginPlay`
  (bind _speedmultiplier (`self.SpeedMultiplier`))
  (set `self.SpeedV` (`KismetMathLibrary.MakeVector` (* (`self.RandomlyNegate` (`KismetMathLibrary.RandomFloatInRange` (`self.MinSpeed`) (`self.MaxSpeed`))) _speedmultiplier) 0.0 (* _speedmultiplier (`self.RandomlyNegate` (`KismetMathLibrary.RandomFloatInRange` (`self.MinSpeed`) (`self.MaxSpeed`)))))))

(event `self.ReceiveTick`
  (params (DeltaSeconds :type "Float (single-precision)"))
  (bind (_returnvalue_x _returnvalue_y _returnvalue_z) (`KismetMathLibrary.BreakVector` (`self.K2_GetActorLocation`)))
  (bind (_speedv_x _speedv_y _speedv_z) (`KismetMathLibrary.BreakVector` (`self.SpeedV`)))
  (`self.K2_AddActorLocalOffset` (* (`self.SpeedV`) DeltaSeconds) true)
  (if (> _returnvalue_z 500.0)
    (set `self.SpeedV` (`KismetMathLibrary.MakeVector` _speedv_x 0.0 (* -1 _speedv_z)) :!label _label)
    (elif (< _returnvalue_z -500.0)
      (goto _label))))

(event `self.SphereMesh.OnComponentHit`
  (params (HitComponent :type "PrimitiveComponent Object Reference") (OtherActor :type "Actor Object Reference") (OtherComp :type "PrimitiveComponent Object Reference") (NormalImpulse :type "Vector Structure") (Hit :type "HitResult Structure (by ref)"))
  (bind (_speedv_x _speedv_y _speedv_z) (`KismetMathLibrary.BreakVector` (`self.SpeedV`)))
  (cast `/Game/Blueprints/BP_Paddles` OtherActor
    (:`then`
      (set `self.SpeedV` (`KismetMathLibrary.MakeVector` (* -1 _speedv_x) 0.0 _speedv_z)))
    (:`CastFailed`
      (`KismetSystemLibrary.PrintString` "Cast Failed!!"))))

(fn `UserConstructionScript`)