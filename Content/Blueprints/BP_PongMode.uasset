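; BP_PongMode is the mode Blueprint for a Pong game, tracking both players' points and showing them on screen.
; On BeginPlay it creates the WBP_UI widget, adds it to the viewport and keeps a reference.
; IncreaseP1Score and IncreaseP2Score each increment that player's points and pass both totals to the widget's UpdateScores.
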(event `self.ReceiveBeginPlay`
  (bind _returnvalue (`|CreateWidget` "/Game/Blueprints/WBP_UI.WBP_UI_C"))
  (`UserWidget.AddToViewport` _returnvalue 0)
  (set `self.WBP_UI` _returnvalue))

(fn `IncreaseP1Score`
  (bind _result (`/Engine/EditorBlueprintResources/StandardMacros.IncrementInt` (`self.P1Points`))
    (:`  `
      (`/Game/Blueprints/WBP_UI.UpdateScores` (`self.WBP_UI`) _result (`self.P2Points`)))))

(fn `IncreaseP2Score`
  (bind _result (`/Engine/EditorBlueprintResources/StandardMacros.IncrementInt` (`self.P2Points`))
    (:`  `
      (`/Game/Blueprints/WBP_UI.UpdateScores` (`self.WBP_UI`) (`self.P1Points`) _result))))

(fn `UserConstructionScript`)